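; VR bow actor that uses a slider component as the grippable draw.
; Gripping the slider plays a timeline that fades in the arrow's material opacity; dropping it waits briefly, then hides the arrow and resets the slider.
; Projectile spawning from the ArrowForSpawn transform is disconnected, as is the speed calculation from slider progress, so releasing the slider fires nothing in this graph.
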(event OnGripped(VRSlider)
  (params (GrippingController :type Grip%20Motion%20Controller%20Component%20Object%20Reference) (GripInformation :type BP%20Actor%20Grip%20Information%20Structure%20%28by%20ref%29))
  (bind _blendingin (Timeline|Timeline PlayFromStart)
    (:Update
      (Rendering|Material|SetScalarParameterValueonMaterials (Variables|Default|Getarrow) "Opacity" _blendingin))))

(event OnDropped(VRSlider)
  (params (GrippingController :type Grip%20Motion%20Controller%20Component%20Object%20Reference) (GripInformation :type BP%20Actor%20Grip%20Information%20Structure%20%28by%20ref%29) (bWasSocketed :type Boolean))
  (Utilities|FlowControl|Sequence
    (:then_0
      (Utilities|FlowControl|Delay 0.02)
      (Rendering|Material|SetScalarParameterValueonMaterials (Variables|Default|Getarrow) "Opacity" 0.0)
      (Class|VRSliderComponent|SetSliderProgress (Variables|Default|GetVRSlider) 0.0))))

(event EventBeginPlay)

(event Collision|EventActorBeginOverlap
  (params (OtherActor :type Actor%20Object%20Reference)))

(event EventTick
  (params (DeltaSeconds :type Float%20%28single-precision%29)))

(fn ConstructionScript)